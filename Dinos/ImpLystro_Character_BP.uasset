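; Character Blueprint for the Imp Lystro dino, which teammates can pet to give it an XP buff.
; A "Pet It" multi-use entry appears for the same team when it is a conscious non-baby without a Buff_XPLystro-type buff.
; Using it adds Buff_XPImpLystro to the dino and plays a replicated random pet montage alongside the player's pickup montage.
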(fn ConstructionScript
  (|CallParentFunction))

(fn BPGetMultiUseEntries
  (params (ForPC :type Player%20Controller%20Object%20Reference) (MultiUseEntries :type Array%20of%20Multi%20Use%20Entry%20Structures))
  (if (== (Variables|/Script/Engine.Actor|GetTargetingTeam ForPC) (Variables|Default|GetTargetingTeam))
    (bind _result (CallFunction|HasXPBuff))
    (if (Math|Boolean|ANDBoolean (not _result) (not (Variables|Default|GetbIsBaby)) (Class|PrimalCharacter|BPIsConscious))
      (Utilities|Array|Add MultiUseEntries (Utilities|Struct|MakeMultiUseEntry 0 "Pet It" 367 10000 false false false false true))))
  (return MultiUseEntries))

(fn HasXPBuff
  (bind _array_element (Utilities|Array|ForEachLoopwithBreak (Class|PrimalCharacter|GetBuffs) :!label _label)
    (:LoopBody
      (Utilities|Casting|CastToBuff_XPLystro _array_element)
      (LocalVariables|SetRetVal true)
      (goto _label Break))
    (:Completed
      (return (LocalVariables|GetRetVal)))))

(fn BPTryMultiUse
  (params (ForPC :type Player%20Controller%20Object%20Reference) (UseIndex :type Integer))
  (bind _petanims (Variables|Default|GetPetAnims))
  (switch int UseIndex
    (:Default
      (return true))
    (:367
      (Class|PrimalBuff|StaticAddBuff "/Game/Mods/ImpLystro/Buffs/Buff_XPImpLystro.Buff_XPImpLystro_C" self 0 0 false)
      (Utilities|FlowControl|Sequence
        (:then_0
          (Class|PrimalCharacter|PlayAnimEx (Utilities|Array|Get(acopy) _petanims (Math|Random|RandomIntegerinRange 0 (- (Utilities|Array|Length _petanims) 1))) 1.0 "None" true false false true)
          (bind _asshooterplayercontroller (Utilities|Casting|CastToShooterPlayerController ForPC))
          (Class|PrimalCharacter|PlayAnimEx (Class|ShooterPlayerController|GetPlayerCharacter _asshooterplayercontroller) "/Game/PrimalEarth/Human/Male/Animations/Human-Pickup_Montage.Human-Pickup_Montage" 1.0 "None" true true false false))
        (:then_1
          (return true))))))